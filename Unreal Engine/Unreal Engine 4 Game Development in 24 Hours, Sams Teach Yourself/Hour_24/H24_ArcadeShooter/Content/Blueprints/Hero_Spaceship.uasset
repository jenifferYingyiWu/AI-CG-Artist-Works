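; Player spaceship that moves by device tilt or a MoveRight axis and fires Plasma_Bolt actors.
; Tick turns the motion-sensor gravity vector, masked by the actor's right vector, into movement input.
; The Shoot action fires once, while holding a touch repeats Shoot on a looping timer.
; A first hit starts damage particles until healed; a second explodes and hides the ship, then calls the GameMode's GoToMainMenu after a delay.
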(event `self.ReceiveTick`
  (params (DeltaSeconds :type "Float (single-precision)"))
  (bind _output_get (set `self.Internal Gravity Vector` (* (`KismetMathLibrary.Normal` (`.Gravity` (`PlayerController.GetInputMotionState` (`GameplayStatics.GetPlayerController` 0)))) (`self.GetActorRightVector`))))
  (if (> (`KismetMathLibrary.VSize` _output_get) 0.1)
    (`self.AddMovementInput` (`self.Internal Gravity Vector`) 2.0)))

(event `self.ReceiveActorBeginOverlap`
  (params (OtherActor :type "Actor Object Reference")))

(event `InputAction|Shoot`
  (params (Key :type "Key Structure" :default "AnyKey"))
  (:`Pressed`
    (`self.Shoot`)))

(event `InputTouch`
  (params (Location :type "Vector Structure") (FingerIndex :type "ETouchIndex Enum"))
  (:`Pressed`
    (bind _returnvalue (`KismetSystemLibrary.K2_SetTimer` null "Shoot" 0.1 true))
    (set `self.ShootTimerHandle` _returnvalue))
  (:`Released`
    (`KismetSystemLibrary.K2_ClearTimerHandle` (`self.ShootTimerHandle`))))

(event `InputAxis|MoveRight`
  (params (AxisValue :type "Float (single-precision)"))
  (`self.MoveRight` AxisValue))

(fn `Heal Damage`
  (set `self.Is Damaged` false)
  (`ActorComponent.Deactivate` (`self.Damage Particle System`)))

(fn `On Death`
  (`GameplayStatics.SpawnEmitterAtLocation` "/Game/StarterContent/Particles/P_Explosion.P_Explosion" (`self.K2_GetActorLocation`))
  (set `self.Is Dead` true)
  (`self.SetActorHiddenInGame` true)
  (`self.SetActorEnableCollision` false)
  (`KismetSystemLibrary.K2_SetTimer` (`GameplayStatics.GetGameMode`) "GoToMainMenu" 3.0))

(fn `Shoot`
  (if (not (`self.Is Dead`))
    (`|SpawnActorFromClass` "/Game/Blueprints/Plasma_Bolt.Plasma_Bolt_C" (`self.GetTransform`) "Undefined" "OverrideRootScale")))

(fn `Take Damage`
  (if (`self.Is Damaged`)
    (`self.On Death`)
    (else
      (set `self.Is Damaged` true)
      (`ActorComponent.Activate` (`self.Damage Particle System`) false))))

(fn `UserConstructionScript`)