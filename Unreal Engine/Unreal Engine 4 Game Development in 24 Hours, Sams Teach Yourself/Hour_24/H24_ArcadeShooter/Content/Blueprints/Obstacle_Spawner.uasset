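; Obstacle spawner actor that periodically spawns either an Asteroid or a Health_Pickup at its own transform.
; BeginPlay starts a one-shot timer with a random delay between SpawnTimeMin and SpawnTimeMax that calls Spawn.
; Spawn picks the health pickup when a random roll falls below HealthPickupProbability, otherwise an asteroid, then re-arms the timer with a new random delay for irregular, endless spawning.
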(event `self.ReceiveBeginPlay`
  (`KismetSystemLibrary.K2_SetTimer` null "Spawn" (`KismetMathLibrary.RandomFloatInRange` (`self.Spawn Time Min`) (`self.Spawn Time Max`))))

(event `self.ReceiveActorBeginOverlap`
  (params (OtherActor :type "Actor Object Reference")))

(event `self.ReceiveTick`
  (params (DeltaSeconds :type "Float (single-precision)")))

(fn `Spawn`
  ;[1 1 1] Should Spawn Health_Pickup
  (if (< (`KismetMathLibrary.RandomFloat`) (`self.Health Pickup Probability`))
    (`|SpawnActorFromClass` "/Game/Blueprints/Health_Pickup.Health_Pickup_C" (`self.GetTransform`) "Undefined" "OverrideRootScale")
    (else
      (`|SpawnActorFromClass` "/Game/Blueprints/Asteroid.Asteroid_C" (`self.GetTransform`) "Undefined" "OverrideRootScale")))
  (`KismetSystemLibrary.K2_SetTimer` null "Spawn" (`KismetMathLibrary.RandomFloatInRange` (`self.Spawn Time Min`) (`self.Spawn Time Max`))))

(fn `UserConstructionScript`)