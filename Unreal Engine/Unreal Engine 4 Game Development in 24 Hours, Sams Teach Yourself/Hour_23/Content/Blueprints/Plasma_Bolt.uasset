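; Plasma Bolt is a projectile actor that destroys what it overlaps, ignoring the player pawn.
; On overlap it spawns an explosion emitter and sound at its own location, then casts the player pawn to Hero_Spaceship to update the score.
; It then destroys the other actor and itself, both only if that cast succeeds.
; BeginPlay and Tick are unused, and no movement logic appears in the graphs.
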(event `self.ReceiveBeginPlay`)

(event `self.ReceiveActorBeginOverlap`
  (params (OtherActor :type "Actor Object Reference"))
  (bind _returnvalue (`self.K2_GetActorLocation`))
  (if (!= OtherActor (`GameplayStatics.GetPlayerPawn` 0))
    (`GameplayStatics.SpawnEmitterAtLocation` "/Game/StarterContent/Particles/P_Explosion.P_Explosion" _returnvalue)
    (`GameplayStatics.PlaySoundAtLocation` "/Game/StarterContent/Audio/Explosion_Cue.Explosion_Cue" _returnvalue)
    (bind _ashero_spaceship (cast `/Game/Blueprints/Hero_Spaceship` (`GameplayStatics.GetPlayerPawn` 0)))
    (`/Game/Blueprints/Hero_Spaceship.UpdateScore` _ashero_spaceship)
    (`self.K2_DestroyActor` OtherActor)
    (`self.K2_DestroyActor`)))

(event `self.ReceiveTick`
  (params (DeltaSeconds :type "Float (single-precision)"))
  (`parent.ReceiveTick` 0.0))

(fn `UserConstructionScript`
  (`parent.UserConstructionScript`))