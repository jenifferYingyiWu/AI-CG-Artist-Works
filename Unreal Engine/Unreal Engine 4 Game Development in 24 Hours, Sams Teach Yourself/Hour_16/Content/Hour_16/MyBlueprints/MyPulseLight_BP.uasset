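; Point light Blueprint that pulses by continually drifting between random brightness levels.
; Each Tick moves the light's intensity toward a target at the constant PulseRate using FInterpToConstant.
; When intensity exactly equals the target, it picks a new random target between MinIntensity and MaxIntensity.
; The construction script is empty, so all behavior runs in Tick.
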(event `self.ReceiveTick`
  (params (DeltaSeconds :type "Float (single-precision)"))
  (if (== (`LightComponentBase.Intensity` (`self.PointLightComponent`)) (`self.Target_intesity`))
    ;[1 1 1] Randomly generate a new target light intensity based on min and max range
    (set `self.Target_intesity` (`KismetMathLibrary.RandomFloatInRange` (`self.min Intensity`) (`self.Max Intensity`)))
    (else
      ;[1 1 1] sets the intensity of the light
      (`LightComponent.SetIntensity` (`self.PointLightComponent`) (`KismetMathLibrary.FInterpTo_Constant` (`LightComponentBase.Intensity` (`self.PointLightComponent`)) (`self.Target_intesity`) DeltaSeconds (`self.PulseRate`))))))

(fn `UserConstructionScript`)