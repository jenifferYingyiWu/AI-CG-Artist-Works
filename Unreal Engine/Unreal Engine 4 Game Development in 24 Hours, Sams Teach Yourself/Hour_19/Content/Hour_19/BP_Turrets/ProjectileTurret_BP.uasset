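; Projectile turret Blueprint that tracks an actor entering its range sphere and fires projectiles at it.
; Each tick it either eases toward the target while a line trace confirms sight, or wanders between random look directions when inactive.
; Once nearly aligned, a DoOnce gate runs reload audio, muzzle effect, projectile spawn and fire-rate delay before resetting.
; The construction script applies range to the trigger and trace endpoint and assigns the reload sound.
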(event `self.TouchTrigger.OnComponentBeginOverlap`
  (params (OtherActor :type "Actor Object Reference") (OtherComp :type "PrimitiveComponent Object Reference") (OtherBodyIndex :type Integer) (bFromSweep :type Boolean) (SweepResult :type "HitResult Structure (by ref)"))
  ;[1 1 1] when an actor enter the touch trigger store the actor in an acot variable and activate the turret
  (set `self.TargetActor` OtherActor)
  (set `self.Activate` true))

(event `self.TouchTrigger.OnComponentEndOverlap`
  (params (OtherActor :type "Actor Object Reference") (OtherComp :type "PrimitiveComponent Object Reference") (OtherBodyIndex :type Integer))
  ;[1 1 1] if the target actor leaves the touch trigger deactivat the turret tracking
  (if (== OtherActor (`self.TargetActor`))
    (set `self.Activate` false)
    (`self.Get New Look Direction`)))

(event `self.ReceiveTick`
  (params (DeltaSeconds :type "Float (single-precision)"))
  (set `self.TheDelta` DeltaSeconds)
  (if (`self.Activate`)
    (`self.Track Target Actor`)
    (else
      (`self.randomLookDirection`))))

(event `Track Target Actor`
  (bind _returnvalue (`KismetMathLibrary.RInterpTo` (`SceneComponent.K2_GetComponentRotation` (`self.Turret_Body`)) (`KismetMathLibrary.FindLookAtRotation` (`SceneComponent.K2_GetComponentLocation` (`self.Turret_Body`)) (`self.K2_GetActorLocation` (`self.TargetActor`))) (`self.TheDelta`) (`self.TrackSpeed`)))
  ;[1 1 1] If target actor has entered the trigger volume then check if there is a clear line of sight
  (bind _outhit (`KismetSystemLibrary.LineTraceSingleForObjects` (`SceneComponent.K2_GetComponentLocation` (`self.Turret_Body`)) (`self.K2_GetActorLocation` (`self.TargetActor`)) (`self.blockingActors`) true))
  (if (== (`.HitActor` (`GameplayStatics.BreakHitResult` _outhit)) (`self.TargetActor`))
    ;[1 1 1] Track target Actor (the actor that overlaped the touch trigger)
    (`SceneComponent.K2_SetWorldRotation` (`self.Turret_Body`) _returnvalue false false)
    (if (== (`SceneComponent.K2_GetComponentRotation` (`self.Turret_Body`)) _returnvalue :`ErrorTolerance` 0.1)
      (`self.FireAtTarget`))))

(event `RandomLookDirection`
  ;[1 1 1] Randomly look around when nor tracking
  (`SceneComponent.K2_SetWorldRotation` (`self.Turret_Body`) (`KismetMathLibrary.RInterpTo` (`SceneComponent.K2_GetComponentRotation` (`self.Turret_Body`)) (`self.TempLookDirection`) (`self.TheDelta`) 1.0) false false)
  ;[1 1 1] check to see if you have gotton to the last random look direction
  (if (== (`SceneComponent.K2_GetComponentRotation` (`self.Turret_Body`)) (`self.TempLookDirection`) :`ErrorTolerance` 5.0)
    (`self.Get New Look Direction`)))

(event `Get New Look Direction`
  ;[1 1 1] Get new random look direction
  (set `self.TempLookDirection` (`KismetMathLibrary.MakeRotator` 0.0 (`KismetMathLibrary.RandomFloatInRange` -10.0 45.0) (`KismetMathLibrary.RandomFloatInRange` -360.0 360.0))))

(event `FireAtTarget`
  ;[1 1 1] Fire Projectile
  (`/Engine/EditorBlueprintResources/StandardMacros.DoOnce` false :!label _label
    (:`Completed`
      (`AudioComponent.Play` (`self.reloadAudio`) 0.0)
      (`KismetSystemLibrary.Delay` (`SoundBase.Duration` (`self.ReloadSound`)))
      (`GameplayStatics.PlaySoundAtLocation` "/Game/StarterContent/Audio/Explosion01.Explosion01")
      (`GameplayStatics.SpawnEmitterAtLocation` (`self.Muzzle FX`) (`SceneComponent.K2_GetComponentLocation` (`self.TraceStart`)) (struct)) ; Muzzle flash
      (`|SpawnActorFromClass` (`self.Projectile`) (`SceneComponent.K2_GetComponentToWorld` (`self.TraceStart`)) "AlwaysSpawn" "OverrideRootScale")
      (`KismetSystemLibrary.Delay` (`self.FireRate`))
      (goto _label :!via `Reset`))))

(fn `UserConstructionScript`
  (`|ExecutionSequence`
    (:`then_0`
      (`SphereComponent.SetSphereRadius` (`self.TouchTrigger`) (`self.TurretRange`) true)
      (`SceneComponent.K2_AddWorldOffset` (`self.TraceEnd`) (`KismetMathLibrary.MakeVector` (`self.TurretRange`)) false false))
    (:`then_1`
      (`AudioComponent.SetSound` (`self.reloadAudio`) (`self.ReloadSound`)))))