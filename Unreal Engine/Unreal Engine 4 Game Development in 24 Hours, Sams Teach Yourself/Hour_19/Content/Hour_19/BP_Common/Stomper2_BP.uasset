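; Stomper hazard that cycles a mesh between its start and a vertically offset destination, damaging actors that overlap its sphere.
; BeginPlay, MoveDestination and Return form an endless loop of eased MoveComponentTo moves and delays, optionally starting at the destination.
; Smoke and stone-hit sound play on each return to start and each overlap.
; The construction script derives the destination from Distance, positions a destination preview mesh and applies an optional StomperMesh override.
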(event `self.ReceiveBeginPlay`
  (if (`self.Start_At_Destination`)
    (`SceneComponent.K2_SetRelativeTransform` (`self.PlatformMesh`) (`self.DestinationTransform`) false false)
    (`self.Return`)
    (else
      (`KismetSystemLibrary.MoveComponentTo` (`self.PlatformMesh`) (.location (`self.DestinationTransform`)) (.rotation (`self.DestinationTransform`)) true true (`self.ReturnSpeed`) :!label _label)
      (`KismetSystemLibrary.Delay` (`self.DestinationDelay`))
      (`KismetSystemLibrary.Delay` (`self.HangDelay`))
      (`self.Return`))))

(event `MoveDestination`
  (goto _label))

(event `Return`
  (`KismetSystemLibrary.MoveComponentTo` (`self.PlatformMesh`) (.location (`self.StartTransForm`)) (.rotation (`self.StartTransForm`)) true true (`self.MoveSpeed`))
  (`self.HitFX`)
  (`KismetSystemLibrary.Delay` (`self.ReturnDelay`))
  (`self.MoveDestination`))

(event `self.Sphere.OnComponentBeginOverlap`
  (params (OtherActor :type "Actor Object Reference") (OtherComp :type "PrimitiveComponent Object Reference") (OtherBodyIndex :type Integer) (bFromSweep :type Boolean) (SweepResult :type "HitResult Structure (by ref)"))
  (`GameplayStatics.ApplyDamage` OtherActor (`self.DamageAmount`) null self)
  (`self.HitFX`))

(event `HitFX`
  (bind _returnvalue (`SceneComponent.K2_GetComponentLocation` (`self.PlatformMesh`)))
  (`GameplayStatics.SpawnEmitterAtLocation` "/Game/Hour_19/Particles/Smoke_puff.Smoke_puff" _returnvalue)
  (`GameplayStatics.PlaySoundAtLocation` "/Game/Hour_19/Audio/StoneHit.StoneHit" _returnvalue))

(fn `UserConstructionScript`
  (bind _returnvalue (`SceneComponent.GetRelativeTransform` (`self.PlatformMesh`)))
  (`|ExecutionSequence`
    (:`then_0`
      (set `self.StartTransForm` _returnvalue)
      (bind _output_get (set `self.DestinationTransform` (`KismetMathLibrary.MakeTransform` (`KismetMathLibrary.MakeVector` (.x (.location _returnvalue)) (.y (.location _returnvalue)) (+ (.z (.location _returnvalue)) (`self.Distance`))) (.rotation _returnvalue) (.scale _returnvalue))))
      (`SceneComponent.K2_SetRelativeTransform` (`self.DestinationMesh`) _output_get false false))
    (:`then_1`
      (if (not (== (`self.StomperMesh`) null))
        (`StaticMeshComponent.SetStaticMesh` (`self.PlatformMesh`) (`self.StomperMesh`))
        (`StaticMeshComponent.SetStaticMesh` (`self.DestinationMesh`) (`self.StomperMesh`))))))