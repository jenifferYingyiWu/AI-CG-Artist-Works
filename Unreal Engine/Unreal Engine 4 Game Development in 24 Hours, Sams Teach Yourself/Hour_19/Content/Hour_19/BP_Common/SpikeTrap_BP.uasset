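; Spike trap Blueprint that springs a bar of spikes upward when its trigger is overlapped, then retracts and re-arms.
; A DoOnce gates the trigger, which plays an activation sound and waits out its length before springing.
; One timeline drives the bar's relative height, playing forward and reverse at separate speeds with short pauses before retracting and re-arming.
; A separate damage sphere applies damage to any actor that begins overlapping it.
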(event `self.DMGSphere.OnComponentBeginOverlap`
  (params (OtherActor :type "Actor Object Reference") (OtherComp :type "PrimitiveComponent Object Reference") (OtherBodyIndex :type Integer) (bFromSweep :type Boolean) (SweepResult :type "HitResult Structure (by ref)"))
  (`GameplayStatics.ApplyDamage` OtherActor (`self.DamageAmount`)))

(event `self.ActivatTrigger.OnComponentBeginOverlap`
  (params (OtherActor :type "Actor Object Reference") (OtherComp :type "PrimitiveComponent Object Reference") (OtherBodyIndex :type Integer) (bFromSweep :type Boolean) (SweepResult :type "HitResult Structure (by ref)"))
  (bind _activationsound (`self.ActivationSound`))
  (`/Engine/EditorBlueprintResources/StandardMacros.DoOnce` false :!label _label
    (:`Completed`
      (`GameplayStatics.PlaySoundAtLocation` _activationsound (`SceneComponent.K2_GetComponentLocation` (`self.Bar`)))
      (`KismetSystemLibrary.Delay` (`SoundBase.Duration` _activationsound))
      (`self.Spring`))))

(event `ResetTriggerBox`
  (goto _label :!via `Reset`))

(event `Spring`
  (`GameplayStatics.PlaySoundAtLocation` (`self.SpringSound`) (`SceneComponent.K2_GetComponentLocation` (`self.Bar`)))
  (`TimelineComponent.SetPlayRate` (`self.Timeline_0`) (`self.SpringSpeed`))
  (bind (_direction _animfloat) (`Timeline|Timeline_0` :!label _label_2)
    (:`Update`
      (`SceneComponent.K2_SetRelativeLocation` (`self.Bar`) (`KismetMathLibrary.MakeVector` 0.0 0.0 (+ (* _animfloat 72.0) -72.0)) false false))
    (:`Finished`
      (switch `ETimelineDirection` _direction
        (:`Forward`
          (`KismetSystemLibrary.Delay` 1.0)
          (`self.ResetSpikes`))
        (:`Backward`
          (`KismetSystemLibrary.Delay` 1.0)
          (`self.ResetTriggerBox`))))))

(event `ResetSpikes`
  (`TimelineComponent.SetPlayRate` (`self.Timeline_0`) (`self.ResetSpeed`))
  (goto _label_2 :!via `ReverseFromEnd`))

(fn `UserConstructionScript`)