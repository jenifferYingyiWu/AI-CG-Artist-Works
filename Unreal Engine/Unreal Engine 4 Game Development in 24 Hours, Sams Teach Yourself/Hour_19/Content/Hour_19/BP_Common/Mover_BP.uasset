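; Mover blueprint for a platform that shuttles endlessly between its start transform and a configurable destination.
; The construction script places DestinationMesh at the destination, caches the platform's start transform and applies optional mesh and material overrides.
; From BeginPlay, MoveDestination and Return call each other in a loop of eased MoveComponentTo moves, each followed by its own delay.
; StartAtDestination snaps the platform to the far end and begins with the return trip.
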(event `self.ReceiveBeginPlay`
  (if (`self.Start_At_Destination`)
    (`SceneComponent.K2_SetRelativeTransform` (`self.PlatformMesh`) (`self.DestinationTransform`) false false)
    (`self.Return`)
    (else
      (`KismetSystemLibrary.MoveComponentTo` (`self.PlatformMesh`) (.location (`self.DestinationTransform`)) (.rotation (`self.DestinationTransform`)) true true (`self.MoveSpeed`) :!label _label)
      (`KismetSystemLibrary.Delay` (`self.DestinationDelay`))
      (`self.Return`))))

(event `MoveDestination`
  (goto _label))

(event `Return`
  (`KismetSystemLibrary.MoveComponentTo` (`self.PlatformMesh`) (.location (`self.StartTransForm`)) (.rotation (`self.StartTransForm`)) true true (`self.MoveSpeed`))
  (`KismetSystemLibrary.Delay` (`self.ReturnDelay`))
  (`self.MoveDestination`))

(fn `UserConstructionScript`
  (`|ExecutionSequence`
    (:`then_0`
      (`SceneComponent.K2_SetRelativeTransform` (`self.DestinationMesh`) (`self.DestinationTransform`) false false)
      (set `self.StartTransForm` (`SceneComponent.GetRelativeTransform` (`self.PlatformMesh`))))
    (:`then_1`
      (if (not (== (`self.Mesh`) null))
        (`StaticMeshComponent.SetStaticMesh` (`self.PlatformMesh`) (`self.Mesh`))
        (`StaticMeshComponent.SetStaticMesh` (`self.DestinationMesh`) (`self.Mesh`))))
    (:`then_2`
      (if (not (== (`self.PlatformMaterial`) null))
        (`PrimitiveComponent.SetMaterial` (`self.PlatformMesh`) 0 (`self.PlatformMaterial`))))))