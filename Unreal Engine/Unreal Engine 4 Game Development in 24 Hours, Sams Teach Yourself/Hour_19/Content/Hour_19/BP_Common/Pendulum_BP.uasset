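; Swinging pendulum hazard that applies HitDamage to any actor overlapping its Box.
; The SwingAnim timeline's update pitches PivotMesh by SwingAmount around a fixed offset, though no Play call starts it in the graph.
; BeginPlay sets the play rate from SwingSpeed, and StartDirection flips the yaw to reverse the swing.
; Taking damage slows the timeline to a near stop for three seconds, with a DoOnce blocking retriggers until speed is restored.
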(event `self.ReceiveBeginPlay`
  (`TimelineComponent.SetPlayRate` (`self.SwingAnim`) (`self.SwingSpeed`))
  (if (`self.Start Direction`)
    (set `self.NewVar_1` -180.0)))

(event `self.ReceiveAnyDamage`
  (params (Damage :type "Float (single-precision)") (DamageType :type "DamageType Object Reference") (InstigatedBy :type "Controller Object Reference") (DamageCauser :type "Actor Object Reference"))
  (`/Engine/EditorBlueprintResources/StandardMacros.DoOnce` false :!label _label
    (:`Completed`
      (`TimelineComponent.SetPlayRate` (`self.SwingAnim`) 0.01)
      (`KismetSystemLibrary.Delay` 3.0)
      (`TimelineComponent.SetPlayRate` (`self.SwingAnim`) (`self.SwingSpeed`))
      (goto _label :!via `Reset`))))

(event `self.Box.OnComponentBeginOverlap`
  (params (OtherActor :type "Actor Object Reference") (OtherComp :type "PrimitiveComponent Object Reference") (OtherBodyIndex :type Integer) (bFromSweep :type Boolean) (SweepResult :type "HitResult Structure (by ref)"))
  (`GameplayStatics.ApplyDamage` OtherActor (`self.HitDamage`) null self))

(fn `UserConstructionScript`)