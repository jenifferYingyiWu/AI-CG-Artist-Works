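; Smasher trap whose two mirrored meshes repeatedly slide apart and slam back, damaging actors that overlap either half's collision.
; Reset and Attack call each other in an endless delayed loop from BeginPlay, easing the retract and playing slide sounds, with a thud and particle burst after each slam.
; The construction script caches the left mesh's position as the slam target and restricts EndLocation to X, which is negated for the right half.
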(event `self.ReceiveBeginPlay`
  (`self.Reset`))

(event `Reset`
  (`GameplayStatics.SpawnSoundAtLocation` "/Game/Hour_19/Audio/Stone_BSlide_Cue.Stone_BSlide_Cue" (`SceneComponent.K2_GetComponentLocation` (`self.P_Explosion`)))
  (`|ExecutionSequence`
    (:`then_0`
      (`KismetSystemLibrary.MoveComponentTo` (`self.SmasherMeshLeft`) (`self.EndLocation`) (struct) true true (`self.ReturnSpeed`))
      (`KismetSystemLibrary.Delay` (`self.AttackDelay`))
      (`self.Attack`))
    (:`then_1`
      (`KismetSystemLibrary.MoveComponentTo` (`self.SmasherMeshRight`) (* (`self.EndLocation`) (-1.0 0.0 0.0)) (struct :`Yaw` 180.0) true true (`self.ReturnSpeed`)))))

(event `Attack`
  (`GameplayStatics.SpawnSoundAtLocation` "/Game/Hour_19/Audio/Stone_FSlide_Cue.Stone_FSlide_Cue" (`SceneComponent.K2_GetComponentLocation` (`self.P_Explosion`)))
  (`|ExecutionSequence`
    (:`then_0`
      (`KismetSystemLibrary.MoveComponentTo` (`self.SmasherMeshLeft`) (`self.StartLocation`) (struct) false false (`self.AttackSpeed`))
      (`GameplayStatics.PlaySoundAtLocation` "/Game/Hour_19/Audio/Thud_Cue.Thud_Cue" (`SceneComponent.K2_GetComponentLocation` (`self.P_Explosion`)))
      (`ActorComponent.Activate` (`self.P_Explosion`) false)
      (`KismetSystemLibrary.Delay` (`self.HitDelay`))
      (`self.Reset`))
    (:`then_1`
      (`KismetSystemLibrary.MoveComponentTo` (`self.SmasherMeshRight`) (`self.StartLocation`) (struct :`Yaw` 180.0) false false (`self.AttackSpeed`)))))

(event `self.DMGCollisionLeft.OnComponentBeginOverlap`
  (params (OtherActor :type "Actor Object Reference") (OtherComp :type "PrimitiveComponent Object Reference") (OtherBodyIndex :type Integer) (bFromSweep :type Boolean) (SweepResult :type "HitResult Structure (by ref)"))
  (`GameplayStatics.ApplyDamage` OtherActor (`self.DamageAmount`) null self))

(event `self.DMGCollisionRight.OnComponentBeginOverlap`
  (params (OtherActor :type "Actor Object Reference") (OtherComp :type "PrimitiveComponent Object Reference") (OtherBodyIndex :type Integer) (bFromSweep :type Boolean) (SweepResult :type "HitResult Structure (by ref)"))
  (`GameplayStatics.ApplyDamage` OtherActor (`self.DamageAmount`) null self))

(fn `UserConstructionScript`
  (bind _x (.x (`self.EndLocation`)))
  (set `self.StartLocation` (`SceneComponent.RelativeLocation` (`self.SmasherMeshLeft`)))
  (if (<= _x -0.1)
    (set `self.EndLocation` (`KismetMathLibrary.MakeVector` _x))
    (else
      (set `self.EndLocation` (0.1 0.0 0.0)))))