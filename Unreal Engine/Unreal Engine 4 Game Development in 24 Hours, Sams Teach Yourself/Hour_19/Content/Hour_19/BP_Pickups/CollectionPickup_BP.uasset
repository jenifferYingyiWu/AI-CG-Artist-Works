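; Collectible pickup Blueprint that sends a collection message with its amount to the actor overlapping its root component.
; A DoOnce gate limits this to one trigger, then hides the mesh and plays sound and particle effects.
; After a delay, if respawning is enabled, it shows the mesh with respawn effects and resets the gate.
; The construction script applies optional mesh and material overrides.
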(event `self.PickUpRoot.OnComponentBeginOverlap`
  (params (OtherActor :type "Actor Object Reference") (OtherComp :type "PrimitiveComponent Object Reference") (OtherBodyIndex :type Integer) (bFromSweep :type Boolean) (SweepResult :type "HitResult Structure (by ref)"))
  (bind _returnvalue (`SceneComponent.K2_GetComponentLocation` (`self.PickUpRoot`)))
  (`/Engine/EditorBlueprintResources/StandardMacros.DoOnce` false :!label _label
    (:`Completed`
      (message `/Game/Hour_19/BP_Levers/Hour_18_BPI.PickupCollection` OtherActor (`self.PickupAmount`))
      (`SceneComponent.SetHiddenInGame` (`self.PickupMesh`) true false)
      (`GameplayStatics.PlaySoundAtLocation` (`self.PickupSound`) _returnvalue)
      (`GameplayStatics.SpawnEmitterAtLocation` (`self.PickupFX`) _returnvalue)
      (`KismetSystemLibrary.Delay` (`self.ReSpawnDelay`))
      (`self.ReSpawnPickup`))))

(event `ResetRespawn`
  (goto _label :!via `Reset`))

(event `ReSpawnPickup`
  (bind _returnvalue (`SceneComponent.K2_GetComponentLocation` (`self.PickUpRoot`)))
  (if (`self.Respawn`)
    (`SceneComponent.SetHiddenInGame` (`self.PickupMesh`) false false)
    (`GameplayStatics.PlaySoundAtLocation` (`self.ReSpawnSound`) _returnvalue)
    (`GameplayStatics.SpawnEmitterAtLocation` (`self.PickupReSpawnFX`) _returnvalue)
    (`self.ResetRespawn`)))

(fn `UserConstructionScript`
  (`|ExecutionSequence`
    (:`then_0`
      (if (not (== (`self.Mesh`) null))
        (`StaticMeshComponent.SetStaticMesh` (`self.PickupMesh`) (`self.Mesh`))))
    (:`then_1`
      (if (not (== (`self.Material`) null))
        (`PrimitiveComponent.SetMaterial` (`self.PickupMesh`) 0 (`self.Material`))))))