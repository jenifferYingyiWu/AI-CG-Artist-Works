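; CheckPoint_BP is a one-shot checkpoint that updates the player's respawn point when something overlaps its box trigger.
; It writes its Arrow's world transform to the spawn transform on either BasicFPSGameMode or Basic3rdPGameMode, whichever cast succeeds.
; The ring then turns green and moves with easing, bracketed by activation and completion sounds and particles, before being destroyed.
; The construction script applies the AnimMesh variable as the ring's mesh.
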(event `self.BoxTrigger.OnComponentBeginOverlap`
  (params (OtherActor :type "Actor Object Reference") (OtherComp :type "PrimitiveComponent Object Reference") (OtherBodyIndex :type Integer) (bFromSweep :type Boolean) (SweepResult :type "HitResult Structure (by ref)"))
  (bind _location (.location (`self.GetTransform`)))
  (bind _rotation (.rotation (`self.GetTransform`)))
  (bind _returnvalue (`SceneComponent.K2_GetComponentToWorld` (`self.Arrow`)))
  (bind _location_2 (.location (`SceneComponent.K2_GetComponentToWorld` (`self.Ring_Mesh`))))
  (`/Engine/EditorBlueprintResources/StandardMacros.DoOnce` false
    (:`Completed`
      (bind _asbasic_fpsgame_mode (cast `/Game/BasicFPSGame/Blueprints/BasicFPSGameMode` (`GameplayStatics.GetGameMode`))
        (:`then`
          (set `/Game/BasicFPSGame/Blueprints/BasicFPSGameMode.SpawnTransform` _returnvalue _asbasic_fpsgame_mode))
        (:`CastFailed`
          (bind _asbasic_3rd_pgame_mode (cast `/Game/Basic3rdPGame/Blueprints/Basic3rdPGameMode` (`GameplayStatics.GetGameMode`)))
          (set `/Game/Basic3rdPGame/Blueprints/Basic3rdPGameMode.SpawnTransfrom` _returnvalue _asbasic_3rd_pgame_mode)))
      (`PrimitiveComponent.SetMaterial` (`self.Ring_Mesh`) 0 "/Game/Hour_19/Materials/Green_Mat.Green_Mat")
      (`GameplayStatics.PlaySoundAtLocation` (`self.ActivationSound`) _location)
      (`GameplayStatics.SpawnEmitterAtLocation` (`self.ActivationParticleFX`) _location _rotation)
      (`KismetSystemLibrary.MoveComponentTo` (`self.Ring_Mesh`) (0.0 0.0 200.0) _rotation true true 2.0)
      (`GameplayStatics.PlaySoundAtLocation` (`self.DoneSound`) _location_2)
      (`GameplayStatics.SpawnEmitterAtLocation` (`self.DoneParticleFX`) _location_2 (.rotation (`SceneComponent.K2_GetComponentToWorld` (`self.Ring_Mesh`))))
      (`ActorComponent.K2_DestroyComponent` (`self.Ring_Mesh`)))))

(fn `UserConstructionScript`
  (if (not (== (`self.animMesh`) null))
    (`StaticMeshComponent.SetStaticMesh` (`self.Ring_Mesh`) (`self.animMesh`))))