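; A lever-activatable stomper trap that cycles a mesh vertically and damages actors that overlap its sphere.
; The StomperAnim timeline drives the mesh's relative Z, alternating play and reverse with hang and reset delays.
; BeginPlay and ActivateActor share a StartOn toggle that starts the loop or blocks its next forward stroke.
; A FlipFlop limits timeline-triggered smoke and stone-hit sound to every second event, while overlaps also trigger them.
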(event `self.ReceiveBeginPlay`
  (`TimelineComponent.SetPlayRate` (`self.StomperAnim`) (`self.Speed`) :!label _label)
  (if (`self.StartOn`)
    (set `self.StartOn` false)
    (`self.PlayStomperAnim`)
    (else
      (set `self.StartOn` true))))

(event `/Game/Hour_19/BP_Levers/Hour_18_BPI.ActivateActor`
  (goto _label))

(event `self.Sphere.OnComponentBeginOverlap`
  (params (OtherActor :type "Actor Object Reference") (OtherComp :type "PrimitiveComponent Object Reference") (OtherBodyIndex :type Integer) (bFromSweep :type Boolean) (SweepResult :type "HitResult Structure (by ref)"))
  (`GameplayStatics.ApplyDamage` OtherActor (`self.DamageAmount`) null self)
  (`self.PlayStomperAnim`)
  (`self.PlayFX`))

(event `PlayStomperAnim`
  (if (not (`self.StartOn`))
    (bind (_direction _stomperfloat) (`Timeline|StomperAnim` :!label _label_2)
      (:`Update`
        (`SceneComponent.K2_SetRelativeLocation` (`self.StomperMesh`) (`KismetMathLibrary.MakeVector` 0.0 0.0 (* _stomperfloat (`self.Distance`))) false false))
      (:`Finished`
        (switch `ETimelineDirection` _direction
          (:`Forward`
            (`KismetSystemLibrary.Delay` (`self.HangDelay`))
            (`self.ReverseStomperAnim`))
          (:`Backward`
            (`KismetSystemLibrary.Delay` (`self.ResetDelay`))
            (`self.PlayStomperAnim`))))
      (:`SpawnHitFX`
        (`/Engine/EditorBlueprintResources/StandardMacros.FlipFlop`
          (:`B`
            (`self.PlayFX`)))))))

(event `ReverseStomperAnim`
  (goto _label_2 :!via `Reverse`))

(fn `PlayFX`
  (bind _returnvalue (`SceneComponent.K2_GetComponentLocation` (`self.StomperMesh`)))
  (`GameplayStatics.SpawnEmitterAtLocation` "/Game/Hour_19/Particles/Smoke_puff.Smoke_puff" _returnvalue)
  (`GameplayStatics.PlaySoundAtLocation` "/Game/Hour_19/Audio/StoneHit.StoneHit" _returnvalue)
  (return))

(fn `UserConstructionScript`)