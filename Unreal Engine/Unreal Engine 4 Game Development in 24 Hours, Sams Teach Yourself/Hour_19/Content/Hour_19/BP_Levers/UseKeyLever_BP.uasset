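; Interactive lever that the player pulls with E to send an activate message to a list of actors.
; Sphere overlap fades a "Press E" billboard by distance through a dynamic material, and box overlap enables input.
; Presses alternate a timeline forward and back to rotate the lever with sounds, messaging the actors when it finishes.
; An optional one-time-use flag disables the lever after its first pull.
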(event `self.Sphere.OnComponentBeginOverlap`
  (params (OtherActor :type "Actor Object Reference") (OtherComp :type "PrimitiveComponent Object Reference") (OtherBodyIndex :type Integer) (bFromSweep :type Boolean) (SweepResult :type "HitResult Structure (by ref)"))
  (set `self.NewVar_0` OtherActor))

(event `self.Sphere.OnComponentEndOverlap`
  (params (OtherActor :type "Actor Object Reference") (OtherComp :type "PrimitiveComponent Object Reference") (OtherBodyIndex :type Integer))
  (set `self.NewVar_0` null)
  (`MaterialInstanceDynamic.SetScalarParameterValue` (`self.MBillboard_DMI`) "Opacity" 0.0))

(event `self.ReceiveTick`
  (params (DeltaSeconds :type "Float (single-precision)"))
  (if (not (== (`self.NewVar_0`) null))
    (`MaterialInstanceDynamic.SetScalarParameterValue` (`self.MBillboard_DMI`) "Opacity" (`KismetMathLibrary.MapRangeClamped` (`self.GetDistanceTo` (`self.NewVar_0`)) 300.0 200.0 0.0 1.0))))

(event `self.Root_BoxCollision.OnComponentBeginOverlap`
  (params (OtherActor :type "Actor Object Reference") (OtherComp :type "PrimitiveComponent Object Reference") (OtherBodyIndex :type Integer) (bFromSweep :type Boolean) (SweepResult :type "HitResult Structure (by ref)"))
  (`self.EnableInput` (`GameplayStatics.GetPlayerController` 0)))

(event `self.Root_BoxCollision.OnComponentEndOverlap`
  (params (OtherActor :type "Actor Object Reference") (OtherComp :type "PrimitiveComponent Object Reference") (OtherBodyIndex :type Integer))
  (`self.DisableInput` (`GameplayStatics.GetPlayerController` 0)))

(event `Key|E`
  (params (Key :type "Key Structure" :default "AnyKey"))
  (bind _returnvalue (`self.K2_GetActorLocation`))
  (:`Pressed`
    (if (`self.LeverActive`)
      (if (`self.OneTimeUse`)
        (set `self.LeverActive` false))
      (`/Engine/EditorBlueprintResources/StandardMacros.FlipFlop`
        (:`A`
          (`GameplayStatics.PlaySoundAtLocation` (`self.ForwardAudio`) _returnvalue)
          (bind (_direction _leverrotation) (`Timeline|MoveLever` :!label _label)
            (:`Update`
              (`SceneComponent.K2_SetRelativeRotation` (`self.Lever_Mesh`) (`KismetMathLibrary.MakeRotator` 0.0 (+ (* _leverrotation 50.0) 90.0)) false false))
            (:`Finished`
              (`GameplayStatics.PlaySoundAtLocation` (`self.ActivateAudio`) (`self.K2_GetActorLocation`))
              (for _array_element (`self.ActorList`)
                (message `/Game/Hour_19/BP_Levers/Hour_18_BPI.ActivateActor` _array_element)))))
        (:`B`
          (`GameplayStatics.PlaySoundAtLocation` (`self.BackAudio`) _returnvalue)
          (goto _label :!via `Reverse`))))))

(fn `UserConstructionScript`
  (bind _returnvalue (`PrimitiveComponent.CreateDynamicMaterialInstance` (`self.MaterialBillboard`) 0 "/Game/Hour_19/Materials/PressE_Mat.PressE_Mat"))
  (bind _output_get (set `self.MBillboard_DMI` _returnvalue))
  (`MaterialInstanceDynamic.SetScalarParameterValue` _output_get "Opacity" 0.0))