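; TouchActivate_BP is a touch-triggered pressure plate that sends ActivateActorMessage to a list of actors.
; The player pawn or tagged actors trigger it, and a timeline lowers the platform while blending its dynamic material color, with sound.
; Tagged physics objects snap to an arrow and are held by a runtime-created PhysicsHandle.
; Unless ActivateOnce is set, ending overlap releases them, reverses the animation and messages the listed actors again.
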(event `self.Box_Collision_Root.OnComponentBeginOverlap`
  (params (OtherActor :type "Actor Object Reference") (OtherComp :type "PrimitiveComponent Object Reference") (OtherBodyIndex :type Integer) (bFromSweep :type Boolean) (SweepResult :type "HitResult Structure (by ref)"))
  (bind _returnvalue (`SceneComponent.K2_GetComponentLocation` (`self.Arrow`)))
  (set `self.TheOtherActor` OtherActor)
  (set `self.TheOtherComponent` OtherComp)
  (if (`self.ActivateOnce`)
    (`/Engine/EditorBlueprintResources/StandardMacros.DoOnce` false
      (:`Completed`
        _)))
  (if (and (== (`self.TheOtherActor`) (`GameplayStatics.GetPlayerPawn` 0)) (`self.PawnActivate`))
    (`self.PlayTrigger` :!label _label)
    (for _array_element (`self.ActorActivateList`) :!label _label_2
      (message `/Game/Hour_19/BP_Levers/Hour_18_BPI.ActivateActor` _array_element))
    (elif (`self.ActorHasTag` (`self.TheOtherActor`) (`self.ActorTag`))
      (if (`SceneComponent.IsSimulatingPhysics` (`self.TheOtherComponent`) "None")
        (`SceneComponent.K2_SetWorldLocation` (`self.TheOtherComponent`) _returnvalue false false)
        (bind _returnvalue_2 (`AddComponent|Physics Handle Component_33`))
        (bind _output_get (set `self.physicsHandle` _returnvalue_2))
        (`PhysicsHandleComponent.SetInterpolationSpeed` _output_get 1000.0)
        (`PhysicsHandleComponent.SetLinearStiffness` _output_get 1000.0)
        (`PhysicsHandleComponent.GrabComponent` _output_get (`self.TheOtherComponent`) "None" _returnvalue true)
        (goto _label)
        (else
          (goto _label))))))

(event `self.Box_Collision_Root.OnComponentEndOverlap`
  (params (OtherActor :type "Actor Object Reference") (OtherComp :type "PrimitiveComponent Object Reference") (OtherBodyIndex :type Integer))
  (if (`self.ActivateOnce`)
    _
    (elif (and (== OtherActor (`GameplayStatics.GetPlayerPawn` 0)) (`self.PawnActivate`))
      (`self.ReverseTrigger` :!label _label_3)
      (goto _label_2)
      (elif (`self.ActorHasTag` OtherActor (`self.ActorTag`))
        (`PhysicsHandleComponent.ReleaseComponent` (`self.physicsHandle`))
        (goto _label_3)))))

(event `PlayTrigger`
  (`GameplayStatics.PlaySoundAtLocation` (`self.TriggerDownSound`) (`self.K2_GetActorLocation`))
  (bind (_direction _blendamount) (`Timeline|tansitionAnim` :!label _label_4)
    (:`Update`
      (`MaterialInstanceDynamic.SetScalarParameterValue` (`self.MatTransition`) "BlendAmount" _blendamount)
      (`SceneComponent.K2_SetRelativeLocation` (`self.Platform`) (`KismetMathLibrary.MakeVector` 0.0 0.0 (+ (* (* _blendamount (`self.MoveDistance`)) -1.0) -30.0)) false false))))

(event `ReverseTrigger`
  (`GameplayStatics.PlaySoundAtLocation` (`self.TriggerUpSound`) (`self.K2_GetActorLocation`))
  (goto _label_4 :!via `Reverse`))

(fn `UserConstructionScript`
  (`|ExecutionSequence`
    (:`then_0`
      (bind _returnvalue (`PrimitiveComponent.CreateDynamicMaterialInstance` (`self.Platform`) 0 null))
      (set `self.MatTransition` _returnvalue)
      (`MaterialInstanceDynamic.SetVectorParameterValue` (`self.MatTransition`) "Color_A" (`self.StartColor`))
      (`MaterialInstanceDynamic.SetVectorParameterValue` (`self.MatTransition`) "Color_B" (`self.EndColor`))
      (`MaterialInstanceDynamic.SetScalarParameterValue` (`self.MatTransition`) "Intensity" (`self.ActivationColorIntensity`)))
    (:`then_1`
      (`SceneComponent.SetHiddenInGame` (`self.Platform`) (`self.HideMeshInGame`) false))
    (:`then_2`
      (if (not (== (`self.Mesh`) null))
        (`StaticMeshComponent.SetStaticMesh` (`self.Platform`) (`self.Mesh`))))))