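; Lockable double stone door that opens and closes as actors enter and leave its trigger box.
; A timeline with configurable speed swings both leaves 90 degrees, reversing to close, with slide and impact sounds.
; While locked, overlaps only play a sound.
; ActivateActor toggles the lock, closing the door on lock and either opening or closing it on unlock, depending on OpenDoorOnUnlock.
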(event `self.ReceiveBeginPlay`
  (`TimelineComponent.SetPlayRate` (`self.DoorAnim`) (`self.DoorSpeed`)))

(event `self.TouchBoxTrigger.OnComponentBeginOverlap`
  (params (OtherActor :type "Actor Object Reference") (OtherComp :type "PrimitiveComponent Object Reference") (OtherBodyIndex :type Integer) (bFromSweep :type Boolean) (SweepResult :type "HitResult Structure (by ref)"))
  (if (`self.DoorLocked`)
    (`GameplayStatics.PlaySoundAtLocation` "/Game/Hour_19/Audio/WeaponChange.WeaponChange" (`self.K2_GetActorLocation`) :!label _label)
    (else
      (`self.OpenDoor`))))

(event `self.TouchBoxTrigger.OnComponentEndOverlap`
  (params (OtherActor :type "Actor Object Reference") (OtherComp :type "PrimitiveComponent Object Reference") (OtherBodyIndex :type Integer))
  (if (`self.DoorLocked`)
    (goto _label)
    (else
      (`self.CloseDoor`))))

(event `/Game/Hour_19/BP_Levers/Hour_18_BPI.ActivateActor`
  (if (`self.DoorLocked`)
    (set `self.DoorLocked` false)
    (if (`self.OpenDoorOnUnlock`)
      (`self.OpenDoor`)
      (else
        (`GameplayStatics.PlaySoundAtLocation` "/Game/Hour_19/Audio/WeaponChange.WeaponChange" (`self.K2_GetActorLocation`) :!label _label_2)
        (`self.CloseDoor`)))
    (else
      (set `self.DoorLocked` true)
      (goto _label_2))))

(event `OpenDoor`
  (`GameplayStatics.PlaySoundAtLocation` "/Game/Hour_19/Audio/Stone_FSlide.Stone_FSlide" (`self.K2_GetActorLocation`))
  (bind (_direction _dooranim) (`Timeline|DoorAnim` :!label _label_3)
    (:`Update`
      (bind _returnvalue (* _dooranim 90.0))
      (`SceneComponent.K2_SetRelativeRotation` (`self.LeftDoor_Mesh`) (`KismetMathLibrary.MakeRotator` 0.0 0.0 (+ (* _returnvalue -1.0) 180.0)) false false)
      (`SceneComponent.K2_SetRelativeRotation` (`self.RightDoor_Mesh`) (`KismetMathLibrary.MakeRotator` 0.0 0.0 _returnvalue) false false))
    (:`Finished`
      (`GameplayStatics.PlaySoundAtLocation` "/Game/Hour_19/Audio/StoneHit.StoneHit" (`self.K2_GetActorLocation`)))))

(event `CloseDoor`
  (`GameplayStatics.PlaySoundAtLocation` "/Game/Hour_19/Audio/Stone_BSlide.Stone_BSlide" (`self.K2_GetActorLocation`))
  (goto _label_3 :!via `Reverse`))

(fn `UserConstructionScript`)