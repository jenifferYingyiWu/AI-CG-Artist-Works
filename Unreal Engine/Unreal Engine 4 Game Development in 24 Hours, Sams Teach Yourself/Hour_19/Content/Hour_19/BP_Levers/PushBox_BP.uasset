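; Pushable box Blueprint that the player slides a fixed distance by pressing E while inside its trigger, which enables and disables input on overlap.
; Four side overlap volumes set the push direction along X or Y, and a Visibility line trace cancels the push if blocked.
; Otherwise a sound plays and the MoveBox timeline offsets the box's relative location without sweep, with a DoOnce blocking repeat presses until reset.
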(event `self.triggerInput.OnComponentBeginOverlap`
  (params (OtherActor :type "Actor Object Reference") (OtherComp :type "PrimitiveComponent Object Reference") (OtherBodyIndex :type Integer) (bFromSweep :type Boolean) (SweepResult :type "HitResult Structure (by ref)"))
  (`self.EnableInput` (`GameplayStatics.GetPlayerController` 0)))

(event `Key|E`
  (params (Key :type "Key Structure" :default "AnyKey"))
  (:`Pressed`
    (`/Engine/EditorBlueprintResources/StandardMacros.DoOnce` false :!label _label
      (:`Completed`
        (`KismetSystemLibrary.PrintString` "Push")
        (bind _hitresult (`self.CheskMoveDirection`))
        (if _hitresult
          (`self.ResetInput`)
          (else
            (set `self.ActiveMoveDirection` (`self.MoveDirection`))
            (bind _output_get (set `self.startLoc` (`SceneComponent.RelativeLocation` (`self.PushBox`))))
            (`GameplayStatics.PlaySoundAtLocation` "/Game/Hour_19/Audio/Stone_BSlide.Stone_BSlide" _output_get)
            (bind (_direction _moveanimation) (`Timeline|MoveBox` :!via `PlayFromStart`)
              (:`Update`
                (`SceneComponent.K2_SetRelativeLocation` (`self.PushBox`) (+ (`self.startLoc`) (* (`self.ActiveMoveDirection`) (* _moveanimation (`self.MoveDistance`)))) false false))
              (:`Finished`
                (`self.ResetInput`)))))))))

(event `ResetInput`
  (goto _label :!via `Reset`))

(event `self.triggerInput.OnComponentEndOverlap`
  (params (OtherActor :type "Actor Object Reference") (OtherComp :type "PrimitiveComponent Object Reference") (OtherBodyIndex :type Integer))
  (`self.DisableInput` (`GameplayStatics.GetPlayerController` 0)))

(event `self.Y_Pos.OnComponentBeginOverlap`
  (params (OtherActor :type "Actor Object Reference") (OtherComp :type "PrimitiveComponent Object Reference") (OtherBodyIndex :type Integer) (bFromSweep :type Boolean) (SweepResult :type "HitResult Structure (by ref)"))
  (set `self.MoveDirection` (0.0 -1.0 0.0)))

(event `self.Y_Neg.OnComponentBeginOverlap`
  (params (OtherActor :type "Actor Object Reference") (OtherComp :type "PrimitiveComponent Object Reference") (OtherBodyIndex :type Integer) (bFromSweep :type Boolean) (SweepResult :type "HitResult Structure (by ref)"))
  (set `self.MoveDirection` (0.0 1.0 0.0)))

(event `self.X_pos.OnComponentBeginOverlap`
  (params (OtherActor :type "Actor Object Reference") (OtherComp :type "PrimitiveComponent Object Reference") (OtherBodyIndex :type Integer) (bFromSweep :type Boolean) (SweepResult :type "HitResult Structure (by ref)"))
  (set `self.MoveDirection` (-1.0 0.0 0.0)))

(event `self.X_Neg.OnComponentBeginOverlap`
  (params (OtherActor :type "Actor Object Reference") (OtherComp :type "PrimitiveComponent Object Reference") (OtherBodyIndex :type Integer) (bFromSweep :type Boolean) (SweepResult :type "HitResult Structure (by ref)"))
  (set `self.MoveDirection` (1.0 0.0 0.0)))

(fn `CheskMoveDirection`
  (returns (HitResult :type Boolean))
  (bind _returnvalue (`SceneComponent.K2_GetComponentLocation` (`self.triggerInput`)))
  (bind (_outhit _returnvalue_2) (`KismetSystemLibrary.LineTraceSingle` :`Start` _returnvalue :`End` (+ _returnvalue (* (`self.MoveDirection`) (`self.MoveDistance`))) :`TraceChannel` "TraceTypeQuery1" :`DrawDebugType` "ForDuration"))
  (return _returnvalue_2))

(fn `UserConstructionScript`)