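; Game mode for the basic FPS that respawns the player after death and keeps an elapsed game timer.
; It saves the character's starting transform and binds to its OnDestroyed event.
; On destruction it waits briefly, spawns and possesses a new character there with sound and particles, then rebinds.
; A looping tenth-second timer rolls counters into seconds and minutes and rebuilds the TimerString text.
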(event `self.ReceiveBeginPlay`
  (`self.Respawn`)
  (`KismetSystemLibrary.K2_SetTimer` null "GameTimer" 0.1 true))

(event `Respawn`
  (bind _returnvalue (`GameplayStatics.GetPlayerCharacter` 0))
  (set `self.SpawnTransform` (`self.GetTransform` _returnvalue))
  (bind _asbasic_fpscharacter (cast `/Game/BasicFPSGame/Blueprints/BasicFPSCharacter` _returnvalue))
  (add `self.OnDestroyed` _asbasic_fpscharacter (delegate `OnDestroyedPlayer`)))

(event `OnDestroyedPlayer`
  (bind _location (.location (`self.SpawnTransform`)))
  (`KismetSystemLibrary.Delay` 2.0)
  (bind _returnvalue (`|SpawnActorFromClass` "/Game/BasicFPSGame/Blueprints/BasicFPSCharacter.BasicFPSCharacter_C" (`self.SpawnTransform`) "Undefined" "OverrideRootScale"))
  (`Controller.Possess` (`GameplayStatics.GetPlayerController` 0) _returnvalue)
  (`GameplayStatics.PlaySoundAtLocation` "/Game/Hour_19/Audio/bong.bong" _location)
  (`GameplayStatics.SpawnEmitterAtLocation` "/Game/Hour_19/Particles/P_Spawn.P_Spawn" _location (.rotation (`self.SpawnTransform`)))
  (`self.Respawn`))

(event `GameTimer`
  (bind _result (`/Engine/EditorBlueprintResources/StandardMacros.IncrementInt` (`self.tenthOFSecond`))
    (:`  `
      (if (> _result 9)
        (set `self.tenthOFSecond` 0)
        (bind _result_2 (`/Engine/EditorBlueprintResources/StandardMacros.IncrementInt` (`self.Seconds`))
          (:`  `
            (if (> _result_2 59)
              (set `self.Seconds` 0)
              (`/Engine/EditorBlueprintResources/StandardMacros.IncrementInt` (`self.Minuts`)
                (:`  `
                  (`self.UpdateString`)))
              (else
                (`self.UpdateString`)))))
        (else
          (`self.UpdateString`))))))

(event `UpdateString`
  (set `self.TimerString` (`KismetStringLibrary.Concat_StrStr` (`KismetStringLibrary.Concat_StrStr` (`KismetStringLibrary.Concat_StrStr` (`KismetStringLibrary.Concat_StrStr` (`KismetStringLibrary.Conv_IntToString` (`self.Minuts`)) " M:") (`KismetStringLibrary.Conv_IntToString` (`self.Seconds`))) " S:") (`KismetStringLibrary.Conv_IntToString` (`self.tenthOFSecond`)))))

(fn `UserConstructionScript`)