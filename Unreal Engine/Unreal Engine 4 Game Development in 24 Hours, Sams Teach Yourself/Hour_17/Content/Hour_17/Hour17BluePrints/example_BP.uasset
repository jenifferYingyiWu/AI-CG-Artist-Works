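; Example construction-script Blueprint that procedurally builds a repeated array of static meshes.
; The Construction Script loops over a component count, adding an arrow component as a pivot whose location and rotation offsets multiply by the loop index.
; Each pass adds a static mesh with a configurable transform, mesh and material, then attaches it to that arrow, yielding linear or radial patterns.
; The event graph holds only disabled default events.
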(fn `UserConstructionScript`
  (locals (tempArrowComp :type "ArrowComponent Object Reference") (tempMeshComp :type "StaticMeshComponent Object Reference"))
  (for _index (range (+ (`self.NumComps`) 1))
    (bind _returnvalue (`AddComponent|NODE_AddArrowComponent-0` :`RelativeTransform` (`KismetMathLibrary.MakeTransform` (* (`self.PivCompLocation`) _index) (* (`self.PivCompRotation `) _index))))
    (set `local.tempArrowComp` _returnvalue)
    (bind _returnvalue_2 (`AddComponent|NODE_AddStaticMeshComponent-0` :`RelativeTransform` (`KismetMathLibrary.MakeTransform` (`self.MeshCompLocation`) (`self.MeshCompRotation`) (`self.MeshCompScale`))))
    (bind _output_get (set `local.tempMeshComp` _returnvalue_2))
    (`StaticMeshComponent.SetStaticMesh` _output_get (`self.SM_MeshAsset`))
    (`SceneComponent.K2_AttachTo` (`local.tempMeshComp`) (`local.tempArrowComp`) "None" "KeepRelativeOffset" true)
    (`PrimitiveComponent.SetMaterial` (`local.tempMeshComp`) 0 (`self.SM_Material`))))