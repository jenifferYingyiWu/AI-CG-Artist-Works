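; Asteroid field spawner that fills a box volume with randomized asteroid actors when play begins.
; The construction script sizes the box from a spawn bounds variable.
; BeginPlay spawns a set count of Asteriod_BP at random points in the box, each with random per-axis scale, spin, drift velocity and a mesh picked from a list.
; Spawns adjust position to avoid collisions and are skipped if still blocked.
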(event `self.ReceiveBeginPlay`
  (bind _box (`self.Box`))
  (bind _min_start_rotation (`self.Min Start Rotation`))
  (bind _max_start_rotation (`self.Max Start Rotation`))
  (bind _mesh_list (`self.Mesh List`))
  (bind _returnvalue (`KismetMathLibrary.RandomFloatInRange` (`self.Min Asteriod Size`) (`self.Max Asteriod Size`)))
  (for _ (range (+ (`self.Number of asteriods`) 1))
    (`|SpawnActorFromClass` "/Game/Blueprints/Asteriod_BP.Asteriod_BP_C" (`KismetMathLibrary.MakeTransform` (`KismetMathLibrary.RandomPointInBoundingBox` (`SceneComponent.K2_GetComponentLocation` _box) (`BoxComponent.BoxExtent` _box)) (struct) (`KismetMathLibrary.MakeVector` _returnvalue _returnvalue _returnvalue)) "AdjustIfPossibleButDontSpawnIfColliding" "OverrideRootScale" null (`KismetMathLibrary.MakeVector` (`KismetMathLibrary.RandomFloatInRange` _min_start_rotation _max_start_rotation) (`KismetMathLibrary.RandomFloatInRange` _min_start_rotation _max_start_rotation) (`KismetMathLibrary.RandomFloatInRange` _min_start_rotation _max_start_rotation)) (`KismetMathLibrary.MakeVector` (`KismetMathLibrary.RandomFloatInRange` -100.0 100.0) (`KismetMathLibrary.RandomFloatInRange` -100.0 100.0) (`KismetMathLibrary.RandomFloatInRange` -100.0 100.0)) (`KismetArrayLibrary.Array_Get` _mesh_list (`KismetMathLibrary.RandomInteger` (`KismetArrayLibrary.Array_Length` _mesh_list))))))

(fn `UserConstructionScript`
  (`BoxComponent.SetBoxExtent` (`self.Box`) (`self.Spawn bounds`) true))