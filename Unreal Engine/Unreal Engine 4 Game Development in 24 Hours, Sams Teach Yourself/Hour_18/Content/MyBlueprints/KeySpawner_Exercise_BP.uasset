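; Key spawner exercise Blueprint: a lever that spawns a physics actor when the player releases E near it.
; Box overlap toggles input for player 0, and ending the overlap also prints a debug string.
; E plays a timeline that pitches the lever mesh, then spawns explosion effects, sound and PhysicActor_BP_TIY_1 at the Arrow component's transform.
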(event `self.Box.OnComponentBeginOverlap`
  (params (OtherActor :type "Actor Object Reference") (OtherComp :type "PrimitiveComponent Object Reference") (OtherBodyIndex :type Integer) (bFromSweep :type Boolean) (SweepResult :type "HitResult Structure (by ref)"))
  (`self.EnableInput` (`GameplayStatics.GetPlayerController` 0)))

(event `self.Box.OnComponentEndOverlap`
  (params (OtherActor :type "Actor Object Reference") (OtherComp :type "PrimitiveComponent Object Reference") (OtherBodyIndex :type Integer))
  (`self.DisableInput` (`GameplayStatics.GetPlayerController` 0))
  (`KismetSystemLibrary.PrintString` "Hello"))

(event `Key|E`
  (params (Key :type "Key Structure" :default "AnyKey"))
  (bind _returnvalue (`SceneComponent.K2_GetComponentToWorld` (`self.Arrow`)))
  (bind _location (.location _returnvalue))
  (:`Released`
    (bind (_direction _leverrotation) (`Timeline|LeverAnim` :!via `PlayFromStart`)
      (:`Update`
        (`SceneComponent.K2_SetRelativeRotation` (`self.LeverMesh`) (`KismetMathLibrary.MakeRotator` 0.0 (* _leverrotation 60.0)) false false))
      (:`Finished`
        (`GameplayStatics.SpawnEmitterAtLocation` "/Game/MobileStarterContent/Particles/P_Explosion.P_Explosion" _location (.rotation _returnvalue))
        (`GameplayStatics.PlaySoundAtLocation` "/Game/MobileStarterContent/Audio/Explosion01.Explosion01" _location)
        (`|SpawnActorFromClass` "/Game/TIYs/PhysicActor_BP_TIY_1.PhysicActor_BP_TIY_1_C" _returnvalue "Undefined" "OverrideRootScale")))))

(fn `UserConstructionScript`)