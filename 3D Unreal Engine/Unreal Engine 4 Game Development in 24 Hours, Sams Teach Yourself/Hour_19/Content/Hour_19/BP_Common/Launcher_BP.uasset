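; Launcher actor that throws player 0's character along its forward vector and upward when anything overlaps its Box.
; The overlap activates the Pow sound and an ice explosion particle, then calls LaunchCharacter, overriding current velocity with one built from Distance and Height.
; The construction script applies BaseMesh when set and always assigns LaunchSound to Pow, as its validity check is disconnected.
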(event `self.Box.OnComponentBeginOverlap`
  (params (OtherActor :type "Actor Object Reference") (OtherComp :type "PrimitiveComponent Object Reference") (OtherBodyIndex :type Integer) (bFromSweep :type Boolean) (SweepResult :type "HitResult Structure (by ref)"))
  (`ActorComponent.Activate` (`self.Pow`) false)
  (`ActorComponent.Activate` (`self.P_TraceMagic_AreaIce_Expl`) false)
  (`Character.LaunchCharacter` (`GameplayStatics.GetPlayerCharacter` 0) (+ (* (`self.GetActorForwardVector`) (`self.Distance`)) (`KismetMathLibrary.MakeVector` 0.0 0.0 (`self.Height`))) true true))

(fn `UserConstructionScript`
  (`|ExecutionSequence`
    (:`then_0`
      (if (!= (`self.BaseMesh`) null)
        (`StaticMeshComponent.SetStaticMesh` (`self.LauncherMesh`) (`self.BaseMesh`))))
    (:`then_1`
      (`AudioComponent.SetSound` (`self.Pow`) (`self.LaunchSound`)))))