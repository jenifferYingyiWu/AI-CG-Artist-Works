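; Turret actor that fires bursts of Pattern_projectile_BP from its Arrow component, starting on BeginPlay and repeating indefinitely.
; A self-calling SpawnSequence event runs through a DoN node, waiting SpawnRate before each shot, then pausing for PauseTime and resetting once NumberTospawn is reached.
; Each shot plays a sound and particle effect, passing the turret's size, speed, gravity, bounce, lifespan and hit effect settings to the projectile.
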(event `self.ReceiveBeginPlay`
  (`self.SpawnSequence`))

(event `SpawnSequence`
  (bind _location (.location (`SceneComponent.K2_GetComponentToWorld` (`self.Arrow`))))
  (bind _rotation (.rotation (`SceneComponent.K2_GetComponentToWorld` (`self.Arrow`))))
  (bind _counter (`/Engine/EditorBlueprintResources/StandardMacros.Do N` (`self.NumberTospawn`) :!label _label)
    (:`Exit`
      (set `self.CurrentSpawn` _counter)
      (`KismetSystemLibrary.Delay` (`self.SpawnRate`))
      (`GameplayStatics.PlaySoundAtLocation` "/Game/Hour_19/Audio/Pop.Pop" _location)
      (`GameplayStatics.SpawnEmitterAtLocation` (`self.SpanwEffect`) _location _rotation)
      (`|SpawnActorFromClass` "/Game/Hour_19/BP_Turrets/Pattern_projectile_BP.Pattern_projectile_BP_C" (`KismetMathLibrary.MakeTransform` _location _rotation (`self.ProjectileSize`)) "AlwaysSpawn" "OverrideRootScale" self (`self.EnableBounce`) (`self.ProjectilGravityScale`) (`self.ProjectileSpeed`) (`self.ProjectileHitEffect`) (`self.ProjectileLifeSpan`) (`self.ProjectileBounciness`) 10000.0)
      (if (>= (`self.CurrentSpawn`) (`self.NumberTospawn`))
        (`KismetSystemLibrary.Delay` (`self.PauseTime`))
        (`self.ResetSpawn`)
        (`self.SpawnSequence`)
        (else
          (`self.SpawnSequence`))))))

(event `ResetSpawn`
  (goto _label :!via `Reset`))

(fn `UserConstructionScript`)