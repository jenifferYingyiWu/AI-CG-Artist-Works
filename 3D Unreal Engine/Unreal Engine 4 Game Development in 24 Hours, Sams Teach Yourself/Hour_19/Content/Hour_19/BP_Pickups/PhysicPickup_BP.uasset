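; PhysicPickup_BP is a pickup actor with a configurable mesh and material that can respawn itself when destroyed.
; The construction script applies the optional Mesh and MeshMaterial overrides to the TurretBody component.
; BeginPlay stores the initial transform.
; When RespawnOnDestroy is set, Destroyed spawns a replacement at that transform, passing on the mesh, material and enabled respawn flag so the cycle repeats.
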(event `self.ReceiveBeginPlay`
  (set `self.NewVar_0` (`self.GetTransform`)))

(event `self.ReceiveDestroyed`
  (if (`self.RespawnOnDestroy`)
    (`|SpawnActorFromClass` "PhysicPickup_BP_C" (`self.NewVar_0`) "Undefined" "OverrideRootScale" null (`self.Mesh`) (`self.MeshMaterial`) true)))

(fn `UserConstructionScript`
  (`|ExecutionSequence`
    (:`then_0`
      (if (not (== (`self.Mesh`) null))
        (`StaticMeshComponent.SetStaticMesh` (`self.Turret_Body`) (`self.Mesh`))))
    (:`then_1`
      (if (not (== (`self.MeshMaterial`) null))
        (`PrimitiveComponent.SetMaterial` (`self.Turret_Body`) 0 (`self.MeshMaterial`))))))