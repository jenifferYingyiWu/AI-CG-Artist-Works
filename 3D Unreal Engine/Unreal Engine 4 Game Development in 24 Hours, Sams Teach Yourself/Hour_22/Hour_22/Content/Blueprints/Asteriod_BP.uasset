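; Asteroid actor that drifts and spins through physics once play begins.
; On BeginPlay it adds its AngularRotation and LinearVelocity variables to the current velocities of the SMRock mesh component.
; It then conditionally replaces that component's static mesh with the NewMesh variable, allowing the rock's shape to vary.
; The construction script is empty, so all setup happens at runtime.
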(event `self.ReceiveBeginPlay`
  (bind _new_mesh (`self.New Mesh`))
  (`PrimitiveComponent.SetPhysicsAngularVelocity` (`self.SM_Rock`) (`self.Angular rotation`) true "None")
  (`PrimitiveComponent.SetAllPhysicsLinearVelocity` (`self.SM_Rock`) (`self.Linear Velocity`) true)
  (if (not (== _new_mesh null))
    (`StaticMeshComponent.SetStaticMesh` (`self.SM_Rock`) _new_mesh)))

(fn `UserConstructionScript`)