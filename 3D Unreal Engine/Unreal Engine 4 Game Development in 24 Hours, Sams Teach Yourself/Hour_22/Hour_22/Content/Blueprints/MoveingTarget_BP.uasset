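; Hoop target that can spin and counts hits when something leaves its collision cylinder.
; On begin play, an optional Rotate timeline starts at a set rate with a mover sound, its output scaled by a direction-signed full turn.
; End overlap plays a bong, applies the hit material and updates the count text, gated by a DoOnce with delayed reset.
; Tick smoothly turns the text toward the player without pitch.
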(event `self.ReceiveBeginPlay`
  (`|ExecutionSequence`
    (:`then_0`
      ;[1 1 1] Set the play rate of the time line
      (`TimelineComponent.SetPlayRate` (`self.Rotate`) (`self.RotationRate`))
      ;[1 1 1] Check to see if it should rotate. Start timeline and active sound
      (if (`self.RotateOnOff`)
        (`TimelineComponent.Play` (`self.Rotate`))
        (`ActorComponent.Activate` (`self.MoverSound`) false)))
    (:`then_1`
      ;[1 1 1] Set the rotation direction
      (if (`self.Direction`)
        (set `self.rotation Amount` 360.0)
        (else
          (set `self.rotation Amount` -360.0))))))

(event `self.CollisionCylinder.OnComponentEndOverlap`
  (params (OtherActor :type "Actor Object Reference") (OtherComp :type "PrimitiveComponent Object Reference") (OtherBodyIndex :type Integer))
  (bind _hitcount (`self.HitCount`))
  ;[1 1 1] Only allow the player character to activate once
  (`/Engine/EditorBlueprintResources/StandardMacros.DoOnce` false :!label _label
    (:`Completed`
      (`|ExecutionSequence`
        (:`then_0`
          ;[1 1 1] Count how many times it has been hit and update the textRender component text
          (`GameplayStatics.SpawnSoundAtLocation` "/Game/Blueprints/Audio/bong.bong" (`SceneComponent.K2_GetComponentLocation` (`self.CollisionCylinder`)))
          (`PrimitiveComponent.SetMaterial` (`self.Hoop_Mesh`) 0 (`self.HitMaterial`))
          (`/Engine/EditorBlueprintResources/StandardMacros.IncrementInt` _hitcount
            (:`  `
              (`TextRenderComponent.K2_SetText` (`self.TextRender`) (`KismetTextLibrary.Conv_StringToText` (`KismetStringLibrary.Concat_StrStr` (`self.HitText`) (`KismetStringLibrary.Conv_IntToString` _hitcount)))))))
        (:`then_1`
          (`KismetSystemLibrary.Delay` 3.0)
          (goto _label :!via `Reset`))))))

(event `self.ReceiveTick`
  (params (DeltaSeconds :type "Float (single-precision)"))
  (bind _textrender (`self.TextRender`))
  ;[1 1 1] Make the TextRender Component follow the player
  (set `self.TheDelta` DeltaSeconds)
  (`SceneComponent.K2_SetWorldRotation` (`self.TextRender`) (`KismetMathLibrary.RInterpTo_Constant` (`SceneComponent.K2_GetComponentRotation` _textrender) (`KismetMathLibrary.MakeRotator` (.roll (`KismetMathLibrary.FindLookAtRotation` (`SceneComponent.K2_GetComponentLocation` _textrender) (`self.K2_GetActorLocation` (`GameplayStatics.GetPlayerPawn` 0)))) 0.0 (.yaw (`KismetMathLibrary.FindLookAtRotation` (`SceneComponent.K2_GetComponentLocation` _textrender) (`self.K2_GetActorLocation` (`GameplayStatics.GetPlayerPawn` 0))))) (`self.TheDelta`) 100.0) false false))

(fn `UserConstructionScript`)